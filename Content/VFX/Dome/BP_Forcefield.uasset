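; BP_Forcefield is a dome barrier for a two-player knockback game that shatters when a player hits it hard enough.
; Hits check each player's cached pre-impact speed, or knockback while stunned, against DomeKbLimit.
; A break triggers slow motion, camera zoom and shakes, spawns BP_ExplodingForcefield, relaunches the player, then restores the dome after a delay.
; Any stunned hit spawns knockback-scaled Niagara impacts and animates the material's bounce and edge color.
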(event `ZoomToPlayer1`
  (bind _outactors (`GameplayStatics.GetAllActorsOfClass` "/Game/ThirdPerson/Blueprints/Character/BP_ThirdPersonCharacter.BP_ThirdPersonCharacter_C"))
  (for _array_element _outactors
    _)
  (set `/Game/ThirdPerson/Blueprints/Character/BP_ThirdPersonCharacter.FocusPlayer1or2` 4 _array_element))

(event `self.ReceiveBeginPlay`
  (`KismetSystemLibrary.Delay` 0.1)
  (bind _returnvalue (`GameplayStatics.GetActorOfClass` "/Game/ThirdPerson/Blueprints/Character/BP_ThirdPersonCharacter.BP_ThirdPersonCharacter_C"))
  (set `self.Player1Ref` (`/Game/ThirdPerson/Blueprints/Character/BP_ThirdPersonCharacter.Player1Instance` _returnvalue))
  (set `self.Player2Ref` (`/Game/ThirdPerson/Blueprints/Character/BP_ThirdPersonCharacter.Player2Instance` _returnvalue))
  ; Bounce
  (`self.Show Forcefield`)
  (`TimelineComponent.SetPlayRate` (`self.TL_Bounce`) 1.0))

(event `ZoomToPlayer2`
  (bind _outactors (`GameplayStatics.GetAllActorsOfClass` "/Game/ThirdPerson/Blueprints/Character/BP_ThirdPersonCharacter.BP_ThirdPersonCharacter_C"))
  (for _array_element _outactors
    _)
  (set `/Game/ThirdPerson/Blueprints/Character/BP_ThirdPersonCharacter.FocusPlayer1or2` 5 _array_element))

(event `StopZooming`
  (bind _returnvalue (`GameplayStatics.GetActorOfClass` "/Game/ThirdPerson/Blueprints/BP_StaticCamera.BP_StaticCamera_C"))
  (set `SpringArmComponent.CameraLagSpeed` 3.0 (`/Game/ThirdPerson/Blueprints/BP_StaticCamera.SpringArm` _returnvalue))
  (bind _outactors (`GameplayStatics.GetAllActorsOfClass` "/Game/ThirdPerson/Blueprints/Character/BP_ThirdPersonCharacter.BP_ThirdPersonCharacter_C"))
  (for _array_element _outactors
    _)
  (set `/Game/ThirdPerson/Blueprints/Character/BP_ThirdPersonCharacter.FocusPlayer1or2` 0 _array_element))

(event `Show Forcefield`
  ; Alpha Shader
  (`GameplayStatics.PlaySound2D` "/Game/Sounds/SFX/DomeRecharge.DomeRecharge" 1.0 1.0 0.0 null null)
  (bind (_direction _alpha) (`Timeline|Anim Alpha` :!via `PlayFromStart` :!label _label)
    (:`Update`
      (`MeshComponent.SetScalarParameterValueOnMaterials` (`self.Dome`) "Alpha" _alpha))))

(event `Hide Forcefield`
  ; Alpha Shader
  (goto _label :!via `ReverseFromEnd`))

(event `FreezePlayer`
  (`self.DomeColorChange`)
  (bind _asbp_third_person_character (cast `/Game/ThirdPerson/Blueprints/Character/BP_ThirdPersonCharacter` (`self.CastPlayerRef`)))
  (`self.CameraShake`)
  (if (== _asbp_third_person_character (`/Game/ThirdPerson/Blueprints/Character/BP_ThirdPersonCharacter.Player1Instance` _asbp_third_person_character))
    (`self.ZoomToPlayer1`)
    (else
      (`self.ZoomToPlayer2`)))
  (set `self.SavePlayerLocation` (`self.K2_GetActorLocation` _asbp_third_person_character))
  (set `self.ShakeOn` true)
  (`GameplayStatics.SetGlobalTimeDilation` 0.2)
  (bind (_direction _newtrack_0) (`Timeline|PlayerShake`)
    (:`Update`
      (if (== (`self.ShakeOn`) true)
        (`self.K2_SetActorTransform` _asbp_third_person_character (`KismetMathLibrary.Conv_VectorToTransform` (+ (`self.SavePlayerLocation`) (* _newtrack_0 (`/Game/ThirdPerson/Blueprints/Character/BP_ThirdPersonCharacter.Last2Frames` (`self.CastPlayerRef`))))) false false)
        (`KismetSystemLibrary.Delay` (`self.DomeStunDelay`))
        (set `self.ShakeOn` false)
        (`GameplayStatics.SetGlobalTimeDilation` 1.0)
        (`self.StopZooming`)
        (`KismetSystemLibrary.Delay` (`self.DomeStunDelay`))))))

(event `self.Dome.OnComponentHit`
  (params (HitComponent :type "PrimitiveComponent Object Reference") (OtherActor :type "Actor Object Reference") (OtherComp :type "PrimitiveComponent Object Reference") (NormalImpulse :type "Vector Structure") (Hit :type "HitResult Structure (by ref)"))
  (bind _domekblimit (`self.DomeKbLimit`))
  (bind _domekblimit_2 (`self.DomeKbLimit`))
  (bind _returnvalue (`Pawn.GetMovementComponent` (`self.Player1Ref`)))
  (bind _returnvalue_2 (`Pawn.GetMovementComponent` (`self.Player2Ref`)))
  ; Spawn Niagara System
  (`|ExecutionSequence`
    (:`then_0`
      ; Kuppel platzt erst bei bestimmter Velocity (1 Frame bevor er die Kuppel berührt wird die Velocity genomm)
      (bind _asbp_third_person_character (cast `/Game/ThirdPerson/Blueprints/Character/BP_ThirdPersonCharacter` OtherActor))
      (set `self.CastPlayerRef` _asbp_third_person_character)
      (`|ExecutionSequence`
        (:`then_0`
          (if (>= (`/Game/ThirdPerson/Blueprints/Character/BP_ThirdPersonCharacter.Last2Frames` (`self.Player1Ref`)) _domekblimit)
            (bind _output_get (set `self.SaveVectorP1` (`/Game/ThirdPerson/Blueprints/Character/BP_ThirdPersonCharacter.VelocityVectorLast2Frames` (`self.Player1Ref`))))
            (`self.FreezePlayer`)
            (`KismetSystemLibrary.Delay` (`self.DomeStunDelay`))
            (`self.DomeExplosion`)
            (set `MovementComponent.Velocity` (* _output_get (0.0 1.25 1.25)) _returnvalue)
            (`self.DomeRespawn`)))
        (:`then_1`
          (if (and (> (`/Game/ThirdPerson/Blueprints/Character/BP_ThirdPersonCharacter.Knockback` (`self.Player1Ref`)) _domekblimit) (== (`/Game/ThirdPerson/Blueprints/Character/BP_ThirdPersonCharacter.Last2Frames` (`self.Player1Ref`)) 0.0) (== (`/Game/ThirdPerson/Blueprints/Character/BP_ThirdPersonCharacter.IsStunned` (`self.Player1Ref`)) true))
            (bind _output_get_2 (set `self.SaveVectorP1` (* (`KismetMathLibrary.Normal` (* (- (`self.K2_GetActorLocation` (`self.Player1Ref`)) (`self.K2_GetActorLocation`)) (0.0 1.25 1.25))) (0.0 3000.0 20000.0))))
            (`self.DomeExplosion`)
            (set `MovementComponent.Velocity` _output_get_2 _returnvalue)
            (`self.FreezePlayer`)
            (`self.DomeRespawn`)))
        (:`then_2`
          (`|ExecutionSequence`
            (:`then_0`
              (if (>= (`/Game/ThirdPerson/Blueprints/Character/BP_ThirdPersonCharacter.Last2Frames` (`self.Player2Ref`)) _domekblimit_2)
                (bind _output_get_3 (set `self.SaveVectorP2` (`/Game/ThirdPerson/Blueprints/Character/BP_ThirdPersonCharacter.VelocityVectorLast2Frames` (`self.Player2Ref`))))
                (`self.FreezePlayer`)
                (`KismetSystemLibrary.Delay` (`self.DomeStunDelay`))
                (`self.DomeExplosion`)
                (set `MovementComponent.Velocity` (* _output_get_3 (0.0 1.25 1.25)) _returnvalue_2)
                (`self.DomeRespawn`)))
            (:`then_1`
              (if (and (> (`/Game/ThirdPerson/Blueprints/Character/BP_ThirdPersonCharacter.Knockback` (`self.Player2Ref`)) _domekblimit_2) (== (`/Game/ThirdPerson/Blueprints/Character/BP_ThirdPersonCharacter.Last2Frames` (`self.Player2Ref`)) 0.0) (== (`/Game/ThirdPerson/Blueprints/Character/BP_ThirdPersonCharacter.IsStunned` (`self.Player2Ref`)) true))
                (bind _output_get_4 (set `self.SaveVectorP2` (* (`KismetMathLibrary.Normal` (* (- (`self.K2_GetActorLocation` (`self.Player2Ref`)) (`self.K2_GetActorLocation`)) (0.0 1.25 1.25))) (0.0 3000.0 20000.0))))
                (`self.DomeExplosion`)
                (set `MovementComponent.Velocity` _output_get_4 _returnvalue_2)
                (`self.FreezePlayer`)
                (`self.DomeRespawn`)))))))
    (:`then_1`
      (bind _asbp_third_person_character_2 (cast `/Game/ThirdPerson/Blueprints/Character/BP_ThirdPersonCharacter` OtherActor))
      (if (== (`/Game/ThirdPerson/Blueprints/Character/BP_ThirdPersonCharacter.IsStunned` _asbp_third_person_character_2) true)
        (bind _returnvalue_3 (`NiagaraFunctionLibrary.SpawnSystemAtLocation` "/Game/VFX/Dome/NS_Impact.NS_Impact" Hit_Location))
        (bind _output_get_5 (set `self.NiagaraRef` _returnvalue_3))
        (`FXSystemComponent.SetFloatParameter` _output_get_5 "UserScale" (* (`/Game/ThirdPerson/Blueprints/Character/BP_ThirdPersonCharacter.Knockback` _asbp_third_person_character_2) 0.0005))
        (`NiagaraComponent.SetVariableVec3` _output_get_5 "UserRotate" (`KismetMathLibrary.Conv_RotatorToVector` (`KismetMathLibrary.MakeRotFromXZ` (`KismetMathLibrary.Cross_VectorVector` Hit_ImpactNormal (0.0 0.0 1.0)) Hit_ImpactNormal)))
        (bind (_direction _bounce_alpha) (`Timeline|TL_Bounce` :!via `SetNewTime`)
          (:`Update`
            (`MeshComponent.SetScalarParameterValueOnMaterials` (`self.Dome`) "Bounce Alpha" _bounce_alpha)
            (`self.ChangeColor`)))))))

(event `CameraShake`
  (bind _returnvalue (`InputDeviceLibrary.GetPlayerControllerFromInputDevice` (struct)))
  (`PlayerCameraManager.StartCameraShake` :`self` (`PlayerController.PlayerCameraManager` _returnvalue) :`ShakeClass` "/Game/EnvironmentCamera/BP_CamShake.BP_CamShake_C" :`Scale` 0.1))

(event `DomeExplosion`
  (bind _dome (`self.Dome`))
  (`GameplayStatics.PlaySound2D` "/Game/Sounds/SFX/big-room-kick.big-room-kick" 1.0 1.0 0.0 null null)
  (`GameplayStatics.PlaySound2D` "/Game/Sounds/SFX/glass-breaking.glass-breaking" 1.0 1.0 0.0 null null)
  (`SceneComponent.SetVisibility` _dome false false)
  (`PrimitiveComponent.SetCollisionEnabled` _dome "NoCollision")
  (`|SpawnActorFromClass` "/Game/VFX/Dome/BP_ExplodingForcefield.BP_ExplodingForcefield_C" (`KismetMathLibrary.MakeTransform` (`self.K2_GetActorLocation`)) "AlwaysSpawn" "MultiplyWithRoot" null null))

(event `DomeColorChange`
  (`PrimitiveComponent.CreateDynamicMaterialInstance` (`self.Dome`) 0 "/Game/VFX/Dome/MM_Forcefield.MM_Forcefield" "None")
  (`KismetSystemLibrary.Delay` 2.0)
  (`PrimitiveComponent.CreateDynamicMaterialInstance` (`self.Dome`) 0 "/Game/VFX/Dome/MI_Forcefield01.MI_Forcefield01" "None"))

(event `ChangeColor`
  (`GameplayStatics.PlaySound2D` "/Game/Sounds/SFX/DomeTouch2.DomeTouch2" 1.0 1.0 0.0 null null)
  (bind (_direction _edge_color) (`Timeline|Color Change` :!via `PlayFromStart`)
    (:`Update`
      (`MeshComponent.SetColorParameterValueOnMaterials` (`self.Dome`) "EdgeColor" _edge_color))))

(event `DomeVisibility`
  (bind _dome (`self.Dome`))
  (`SceneComponent.SetVisibility` _dome true false)
  (`PrimitiveComponent.SetCollisionEnabled` _dome "QueryAndPhysics"))

(event `DomeRespawn`
  (`KismetSystemLibrary.Delay` 2.0)
  (`self.DomeVisibility`)
  (`self.Show Forcefield`))

(fn `UserConstructionScript`)
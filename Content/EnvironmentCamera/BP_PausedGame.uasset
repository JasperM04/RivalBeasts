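; Actor that toggles the pause menu and also triggers a camera shake when the third-person character enters its box.
; It enables input from player 0 on BeginPlay so IA_Pause can open WBP_PauseMenu, pausing the game with a cursor and UI-only input.
; Closing removes the widget and restores game-only input.
; The box overlap prints a debug "Hello" and starts BP_CamShake on the player camera manager.
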(event `self.ReceiveBeginPlay`
  (`self.EnableInput` (`GameplayStatics.GetPlayerController` 0)))

(event `Close_PauseMenu`
  (bind _returnvalue (`GameplayStatics.GetPlayerController` 0))
  (`Widget.RemoveFromParent` (stale `Pause_Menu` _pausemenu))
  (set `self.PauseMenu` null)
  (`WidgetBlueprintLibrary.SetInputMode_GameOnly` _returnvalue)
  (set `PlayerController.bShowMouseCursor` false _returnvalue)
  (`GameplayStatics.SetGamePaused` false))

(event `Pause_Menu`
  (bind _returnvalue (`GameplayStatics.GetPlayerController` 0))
  (if (`GameplayStatics.IsGamePaused`)
    (bind _pausemenu (`self.PauseMenu`)
      (:`then`
        (`self.Close_PauseMenu`))
      (:`else`
        (bind _returnvalue_2 (`|CreateWidget` "/Game/UI_UX/WBP_PauseMenu.WBP_PauseMenu_C" :!label _label))
        (bind _output_get (set `self.PauseMenu` _returnvalue_2))
        (`UserWidget.AddToViewport` _output_get 0)
        (set `PlayerController.bShowMouseCursor` true _returnvalue)
        (`WidgetBlueprintLibrary.SetInputMode_UIOnlyEx` _returnvalue (`self.PauseMenu`) "LockAlways")
        (`GameplayStatics.SetGamePaused` true)))
    (else
      (goto _label))))

(event `self.Box.OnComponentBeginOverlap`
  (params (OverlappedComponent :type "PrimitiveComponent Object Reference") (OtherActor :type "Actor Object Reference") (OtherComp :type "PrimitiveComponent Object Reference") (OtherBodyIndex :type Integer) (bFromSweep :type Boolean) (SweepResult :type "HitResult Structure (by ref)"))
  (cast `/Game/ThirdPerson/Blueprints/Character/BP_ThirdPersonCharacter` OtherActor)
  (`KismetSystemLibrary.PrintString` "Hello")
  (bind _returnvalue (`InputDeviceLibrary.GetPlayerControllerFromInputDevice` (struct)))
  (`PlayerCameraManager.StartCameraShake` :`self` (`PlayerController.PlayerCameraManager` _returnvalue) :`ShakeClass` "/Game/EnvironmentCamera/BP_CamShake.BP_CamShake_C"))

(event `EnhancedInput|/Game/ThirdPerson/Input/Actions/IA_Pause`
  (params (ActionValue :type Boolean) (ElapsedSeconds :type "Float (double-precision)") (TriggeredSeconds :type "Float (double-precision)") (InputAction :type "InputAction Object Reference" :default "/Game/ThirdPerson/Input/Actions/IA_Pause.IA_Pause"))
  (:`Triggered`
    (`self.Pause_Menu`)))

(fn `UserConstructionScript`)